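; Planter box actor that grows a chosen produce type and lets it be harvested on interaction.
; Interact on an empty box shows a planted mesh, then chained one-second timers swap meshes through two growth stages to harvestable.
; Interact on a harvestable box resets it and reports the produce type to the BP_ProduceTracker found in the level.
; Only Carrot, Tomato and Blueberry have meshes assigned; other types are blank.
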(event `self.ReceiveBeginPlay`
  (`StaticMeshComponent.SetStaticMesh` (`self.PlanterBox`) "/Game/SarahFolder/PlaterBoxMeshes/SM_PlanterEmpty.SM_PlanterEmpty")
  (set `self.Plantable` true))

(event `/Game/SarahFolder/BPI_Interact.Interact`
  (if (`self.Plantable`)
    (set `self.Plantable` false)
    (`StaticMeshComponent.SetStaticMesh` (`self.PlanterBox`) (select `/Game/SarahFolder/E_Produce` (`self.ProduceTypes`) :`NewEnumerator0` "/Game/SarahFolder/PlaterBoxMeshes/SM_Planted3.SM_Planted3" :`NewEnumerator1` "/Game/SarahFolder/PlaterBoxMeshes/SM_Planted2.SM_Planted2" :`NewEnumerator3` "/Game/SarahFolder/PlaterBoxMeshes/SM_Planted1.SM_Planted1" :!type "StaticMesh Object Reference"))
    (`KismetSystemLibrary.K2_SetTimerDelegate` (delegate `Stage1`) 1.0)
    (elif (`self.Harvestable`)
      (`StaticMeshComponent.SetStaticMesh` (`self.PlanterBox`) "/Game/SarahFolder/PlaterBoxMeshes/SM_PlanterEmpty.SM_PlanterEmpty")
      (bind _returnvalue (`GameplayStatics.GetActorOfClass` "/Game/SarahFolder/BP_ProduceTracker.BP_ProduceTracker_C"))
      (`/Game/SarahFolder/BP_ProduceTracker.Harvest` _returnvalue (`self.ProduceTypes`))
      (set `self.Harvestable` false)
      (set `self.Plantable` true))))

(event `Stage1`
  (`StaticMeshComponent.SetStaticMesh` (`self.PlanterBox`) (select `/Game/SarahFolder/E_Produce` (`self.ProduceTypes`) :`NewEnumerator0` "/Game/SarahFolder/PlaterBoxMeshes/SM_CarrotStage1.SM_CarrotStage1" :`NewEnumerator1` "/Game/SarahFolder/PlaterBoxMeshes/SM_TomatoStage1.SM_TomatoStage1" :`NewEnumerator3` "/Game/SarahFolder/PlaterBoxMeshes/SM_BlueberryStage1.SM_BlueberryStage1" :!type "StaticMesh Object Reference"))
  (`KismetSystemLibrary.K2_SetTimerDelegate` (delegate `Stage2`) 1.0))

(event `Stage2`
  (`StaticMeshComponent.SetStaticMesh` (`self.PlanterBox`) (select `/Game/SarahFolder/E_Produce` (`self.ProduceTypes`) :`NewEnumerator0` "/Game/SarahFolder/PlaterBoxMeshes/SM_CarrotStage2.SM_CarrotStage2" :`NewEnumerator1` "/Game/SarahFolder/PlaterBoxMeshes/SM_TomatoStage2.SM_TomatoStage2" :`NewEnumerator3` "/Game/SarahFolder/PlaterBoxMeshes/SM_BlueberryStage2.SM_BlueberryStage2" :!type "StaticMesh Object Reference"))
  (`KismetSystemLibrary.K2_SetTimerDelegate` (delegate `ProduceHarvestable`) 1.0))

(event `ProduceHarvestable`
  (`StaticMeshComponent.SetStaticMesh` (`self.PlanterBox`) (select `/Game/SarahFolder/E_Produce` (`self.ProduceTypes`) :`NewEnumerator0` "/Game/SarahFolder/PlaterBoxMeshes/SM_CarrotHarvestable.SM_CarrotHarvestable" :`NewEnumerator1` "/Game/SarahFolder/PlaterBoxMeshes/SM_TomatoHarvestable.SM_TomatoHarvestable" :`NewEnumerator3` "/Game/SarahFolder/PlaterBoxMeshes/SM_BlueberryHarvestable.SM_BlueberryHarvestable" :!type "StaticMesh Object Reference"))
  (set `self.Harvestable` true))

(fn `UserConstructionScript`)