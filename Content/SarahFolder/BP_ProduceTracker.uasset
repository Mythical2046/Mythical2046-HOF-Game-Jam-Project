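; BP_ProduceTracker keeps running totals of harvested crops: carrots, tomatoes, potatoes, blueberries, strawberries and onions.
; The Harvest event stores the incoming produce type and tests it through a chain of enum comparisons, adding a fixed per-crop yield to the matching counter.
; Each matched branch then calls CountUpdatedMessage to signal the change.
; The potato branch adds zero, so its total never increases through harvesting.
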(event `Harvest`
  (params (ProduceType :type "/Game/SarahFolder/E_Produce Enum" :default "NewEnumerator0"))
  (bind _output_get (set `self.HarvestedProduce` ProduceType))
  (if (`|EnumEquality` _output_get "NewEnumerator0")
    (set `self.CarrotCount` (+ (`self.CarrotCount`) 3))
    (message `/Game/SarahFolder/BPI_CountUpdated.CountUpdated`)
    (elif (`|EnumEquality` (`self.HarvestedProduce`) "NewEnumerator1")
      (set `self.TomatoCount` (+ (`self.TomatoCount`) 6))
      (message `/Game/SarahFolder/BPI_CountUpdated.CountUpdated`)
      (elif (`|EnumEquality` (`self.HarvestedProduce`) "NewEnumerator2")
        (set `self.PotatoCount` (+ (`self.PotatoCount`) 0))
        (message `/Game/SarahFolder/BPI_CountUpdated.CountUpdated`)
        (elif (`|EnumEquality` (`self.HarvestedProduce`) "NewEnumerator3")
          (set `self.BlueberryCount` (+ (`self.BlueberryCount`) 10))
          (message `/Game/SarahFolder/BPI_CountUpdated.CountUpdated`)
          (elif (`|EnumEquality` (`self.HarvestedProduce`) "NewEnumerator4")
            (set `self.StrawberryCount` (+ (`self.StrawberryCount`) 10))
            (message `/Game/SarahFolder/BPI_CountUpdated.CountUpdated`)
            (elif (`|EnumEquality` (`self.HarvestedProduce`) "NewEnumerator5")
              (set `self.OnionCount` (+ (`self.OnionCount`) 3))
              (message `/Game/SarahFolder/BPI_CountUpdated.CountUpdated`))))))))

(fn `UserConstructionScript`)