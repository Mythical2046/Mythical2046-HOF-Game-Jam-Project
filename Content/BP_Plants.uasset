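; BP_Plants is a plant actor that grows through three stages and is picked up when the third-person character touches it.
; A timer set at BeginPlay starts three chained timelines, with the Tomato mesh swapped to engine placeholder meshes as the first two finish.
; Collider overlap with the character destroys the actor and then calls the Pickup dispatcher, with no check on growth stage.
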(event `self.ReceiveBeginPlay`
  (`KismetSystemLibrary.K2_SetTimerDelegate` (delegate `CustomEvent`) 2.0))

(event `CustomEvent`
  (`Timeline|TL_Grow` :`NewTime` (`self.StageOneGrowTime`) :!via `PlayFromStart`
    (:`Finished`
      (`StaticMeshComponent.SetStaticMesh` (`self.Tomato`) "/Engine/InteractiveToolsFramework/Meshes/GizmoBoxArrowHandle.GizmoBoxArrowHandle")
      (`Timeline|TL_GrowStageTwo` :`NewTime` (`self.StageTwoGrowTime`) :!via `PlayFromStart`
        (:`Finished`
          (`StaticMeshComponent.SetStaticMesh` (`self.Tomato`) "/Engine/EditorMeshes/ArcadeEditorSphere.ArcadeEditorSphere")
          (`Timeline|TL_GrowStageThree` :!via `PlayFromStart`))))))

(event `self.Collider.OnComponentBeginOverlap`
  (params (OverlappedComponent :type "PrimitiveComponent Object Reference") (OtherActor :type "Actor Object Reference") (OtherComp :type "PrimitiveComponent Object Reference") (OtherBodyIndex :type Integer) (bFromSweep :type Boolean) (SweepResult :type "HitResult Structure (by ref)"))
  (cast `/Game/ThirdPerson/Blueprints/BP_ThirdPersonCharacter` OtherActor)
  (`self.K2_DestroyActor`)
  (`self.Pickup`))

(fn `UserConstructionScript`)