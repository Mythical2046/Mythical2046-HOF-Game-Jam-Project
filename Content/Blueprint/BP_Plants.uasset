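; BP_Plants is a plant actor that grows in timed stages and is picked up on overlap by the third-person character.
; OnGrow chains three timelines used as timers, each ending by destroying the actor and spawning BP_Plants at the same transform.
; The later timelines are started on the actor just destroyed, not on the spawned replacement.
; Collider overlap with BP_ThirdPersonCharacter destroys the plant, then calls Pickup.
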(event `OnGrow`
  (`Timeline|TL_Grow` :`NewTime` (`self.StageOneGrowTime`) :!via `PlayFromStart`
    (:`Finished`
      (`self.K2_DestroyActor`)
      (`|SpawnActorFromClass` "BP_Plants_C" (`self.GetTransform`) "Undefined" "MultiplyWithRoot" null null)
      (`Timeline|TL_GrowStageTwo` :`NewTime` (`self.StageTwoGrowTime`) :!via `PlayFromStart`
        (:`Finished`
          (`self.K2_DestroyActor`)
          (`|SpawnActorFromClass` "BP_Plants_C" (`self.GetTransform`) "Undefined" "MultiplyWithRoot" null null)
          (`Timeline|TL_GrowStageThree` :!via `PlayFromStart`
            (:`Finished`
              (`self.K2_DestroyActor`)
              (`|SpawnActorFromClass` "BP_Plants_C" (`self.GetTransform`) "Undefined" "MultiplyWithRoot" null null))))))))

(event `self.Collider.OnComponentBeginOverlap`
  (params (OverlappedComponent :type "PrimitiveComponent Object Reference") (OtherActor :type "Actor Object Reference") (OtherComp :type "PrimitiveComponent Object Reference") (OtherBodyIndex :type Integer) (bFromSweep :type Boolean) (SweepResult :type "HitResult Structure (by ref)"))
  (cast `/Game/ThirdPerson/Blueprints/BP_ThirdPersonCharacter` OtherActor)
  (`self.K2_DestroyActor`)
  (`self.Pickup`))

(fn `UserConstructionScript`)