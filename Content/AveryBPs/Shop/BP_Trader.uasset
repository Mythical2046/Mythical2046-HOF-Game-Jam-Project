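; BP_Trader is a shop trader that opens the shop menu through the HUD when interacted with.
; OnProduceSold handles selling six produce types, from carrots to onions.
; It selects the matching inventory count by produce type and, if above zero, decrements it and adds that type's sell value to the inventory's money.
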(event `OnProduceSold`
  (params (ItemSold :type "/Game/SarahFolder/E_Produce Enum" :default "NewEnumerator0"))
  (bind _inventoryref (`self.InventoryRef`))
  (bind _item_sold (`self.Item Sold`))
  (bind _inventoryref_2 (`self.InventoryRef`))
  (bind _returnvalue (select `/Game/SarahFolder/E_Produce` _item_sold :`NewEnumerator0` (`/Game/SarahFolder/BP_ItemTracker.CarrotCount` _inventoryref_2) :`NewEnumerator1` (`/Game/SarahFolder/BP_ItemTracker.TomatoCount` _inventoryref_2) :`NewEnumerator2` (`/Game/SarahFolder/BP_ItemTracker.PotatoCount` _inventoryref_2) :`NewEnumerator3` (`/Game/SarahFolder/BP_ItemTracker.BlueberryCount` _inventoryref_2) :`NewEnumerator4` (`/Game/SarahFolder/BP_ItemTracker.StrawberryCount` _inventoryref_2) :`NewEnumerator5` (`/Game/SarahFolder/BP_ItemTracker.OnionCount` _inventoryref_2)))
  (set `self.Item Sold` ItemSold)
  (if (> _returnvalue 0)
    (`/Engine/EditorBlueprintResources/StandardMacros.DecrementInt` _returnvalue
      (:`  `
        (set `/Game/SarahFolder/BP_ItemTracker.MoneyCount` (+ (`/Game/SarahFolder/BP_ItemTracker.MoneyCount` _inventoryref) (select `/Game/SarahFolder/E_Produce` _item_sold :`NewEnumerator0` (`self.CarrotSellValue`) :`NewEnumerator1` (`self.TomatoSellValue`) :`NewEnumerator2` (`self.PotatoSellValue`) :`NewEnumerator3` (`self.BlueberrySellValue`) :`NewEnumerator4` (`self.StrawberrySellValue`) :`NewEnumerator5` (`self.OnionSellValue`))) _inventoryref)))))

(event `/Game/SarahFolder/BPI_Interact.Interact`
  (`/Game/SarahFolder/BP_HUD.OpenShopMenu` (`self.HUDRef`)))

(fn `UserConstructionScript`)