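; BP_FoodBank is an interactable food bank that takes all of the tracked produce when used.
; On BeginPlay it caches the BP_ProduceTracker found in the level.
; Interact sums the tracker's six produce counts into FoodInBank, overwriting the previous value, then zeroes those counts.
; It then prints the food bank total as formatted text.
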(event `self.ReceiveBeginPlay`
  (bind _returnvalue (`GameplayStatics.GetActorOfClass` "/Game/SarahFolder/BP_ProduceTracker.BP_ProduceTracker_C"))
  (set `self.ProduceTrakerRef` _returnvalue))

(event `/Game/SarahFolder/BPI_Interact.Interact`
  (bind _producetrakerref (`self.ProduceTrakerRef`))
  (bind _producetrakerref_2 (`self.ProduceTrakerRef`))
  (set `self.FoodInBank` (+ (`/Game/SarahFolder/BP_ProduceTracker.TomatoCount` _producetrakerref) (`/Game/SarahFolder/BP_ProduceTracker.PotatoCount` _producetrakerref) (`/Game/SarahFolder/BP_ProduceTracker.BlueberryCount` _producetrakerref) (`/Game/SarahFolder/BP_ProduceTracker.StrawberryCount` _producetrakerref) (`/Game/SarahFolder/BP_ProduceTracker.CarrotCount` _producetrakerref) (`/Game/SarahFolder/BP_ProduceTracker.OnionCount` _producetrakerref)))
  (set `/Game/SarahFolder/BP_ProduceTracker.OnionCount` 0 _producetrakerref_2)
  (set `/Game/SarahFolder/BP_ProduceTracker.TomatoCount` 0 _producetrakerref_2)
  (set `/Game/SarahFolder/BP_ProduceTracker.StrawberryCount` 0 _producetrakerref_2)
  (set `/Game/SarahFolder/BP_ProduceTracker.CarrotCount` 0 _producetrakerref_2)
  (set `/Game/SarahFolder/BP_ProduceTracker.PotatoCount` 0 _producetrakerref_2)
  (set `/Game/SarahFolder/BP_ProduceTracker.BlueberryCount` 0 _producetrakerref_2)
  (`KismetSystemLibrary.PrintText` (`|FormatText` "The food bank has {num} food" (`self.FoodInBank`))))

(fn `UserConstructionScript`)