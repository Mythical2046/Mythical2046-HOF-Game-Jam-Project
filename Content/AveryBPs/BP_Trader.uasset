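; BP_Trader is a trader that appears intended to buy crops from the player, but its sale logic is currently unwired.
; The Interact event is empty, and the construction script does nothing.
; Disconnected nodes use the ItemSold crop type to select a count in InventoryRef, decrement it if positive and add that crop's sell value to MoneyCount.
; Another disconnected node sets ItemSold to Carrot.
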(event `/Game/SarahFolder/BPI_Interact.Interact`)

(fn `UserConstructionScript`)